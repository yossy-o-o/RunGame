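; Player character Blueprint for a 2D flipbook-animated character that can jump.
; On BeginPlay it detaches the camera with world transforms kept, so the view no longer follows the player.
; The Jump_Space input triggers the standard Character jump.
; Each Tick it switches the sprite between the jump and run flipbooks based on whether the movement component is falling.
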(event EventTick
  (params (DeltaSeconds :type Float%20%28single-precision%29))
  ;[0.15 0.15 0.15 0.5] Player_Flip
  (if (AI|Components|NavMovement|IsFalling (Variables|Character|GetCharacterMovement))
    (Sprite|SetFlipbook (Variables|Default|GetSprite) "/Game/2D_images_uisco/00_player/01_jump/Flip_Player-Jump.Flip_Player-Jump")
    (else
      (Sprite|SetFlipbook (Variables|Default|GetSprite) "/Game/2D_images_uisco/00_player/00_run/Flip_Player_Run.Flip_Player_Run"))))

(event EventBeginPlay
  ;[0.15 0.15 0.15 0.5] Player_Camera
  (Transformation|DetachFromComponent (Variables|Default|GetCamera) "KeepWorld" "KeepWorld" "KeepWorld" true))

(event Input|ActionEvents|InputActionJump_Space
  (params (Key :type Key%20Structure :default "None"))
  ;[0.15 0.15 0.15 0.5] Player_Jump
  (:Pressed
    (Character|Jump)))

(fn ConstructionScript)